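; BP_GM_Main is the main game mode Blueprint that spawns local players at level start.
; On BeginPlay it creates a player for each PlayerStart found, using the array index as the player index.
; Each gets a spawned BP_PlayerCharacter at that start's transform, possessed by player controller 0 for the first and by the created controller for the rest.
; After the loop it calls CallSetUpCamera.
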(event EventBeginPlay
  ;[0.15 0.15 0.15 0.5] For each player spawn, spawn a player and assign the index to the player start, 0 is player 1 , 1 is player 2 etc
  (bind _outactors (Actor|GetAllActorsOfClass "/Script/Engine.PlayerStart"))
  (for (_array_element _array_index) _outactors
    (bind _output_get (Variables|Default|SetIndex _array_index))
    (bind _returnvalue (Class|GameplayStatics|CreatePlayer _output_get))
    (if (> (Variables|Default|GetIndex) 0)
      (bind _returnvalue_2 (Game|SpawnActorfromClass "/Game/MyContent/Player/BP_PlayerCharacter.BP_PlayerCharacter_C" (Transformation|GetActorTransform _array_element) "Undefined" "MultiplyWithRoot" 0 0))
      (Pawn|Possess _returnvalue _returnvalue_2)
      (else
        (bind _returnvalue_3 (Game|SpawnActorfromClass "/Game/MyContent/Player/BP_PlayerCharacter.BP_PlayerCharacter_C" (Transformation|GetActorTransform _array_element) "Undefined" "MultiplyWithRoot" 0 0))
        (Pawn|Possess (Game|GetPlayerController 0) _returnvalue_3))))
  (Default|CallSetUpCamera))

(fn ConstructionScript)