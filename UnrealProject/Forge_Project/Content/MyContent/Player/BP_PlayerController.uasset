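; Player controller that routes Enhanced Input for movement and camera look to the possessed BP_PlayerCharacter.
; On possess it casts and caches the character, then registers the movement and camera mapping contexts through a small AddInput helper.
; Every trigger state of the move action forwards its value to MoveCharacter, while look input goes to RotateCharacter, leaving the actual motion logic in the character.
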(event Input|EnhancedActionEvents|EnhancedInputActionIA_Move
  (params (ActionValue :type Vector%202D%20Structure) (ElapsedSeconds :type Float%20%28double-precision%29) (TriggeredSeconds :type Float%20%28double-precision%29) (InputAction :type Input%20Action%20Object%20Reference :default "/Game/MyContent/Player/Input/IA_Move.IA_Move"))
  (:Triggered
    (Default|MoveCharacter (Variables|Default|GetCharRef) ActionValue :!label _label))
  (:Started
    (goto _label))
  (:Ongoing
    (goto _label))
  (:Canceled
    (goto _label))
  (:Completed
    (goto _label)))

(event Input|EnhancedActionEvents|EnhancedInputActionIA_Look
  (params (ActionValue :type Vector%202D%20Structure) (ElapsedSeconds :type Float%20%28double-precision%29) (TriggeredSeconds :type Float%20%28double-precision%29) (InputAction :type Input%20Action%20Object%20Reference :default "/Game/MyContent/Player/Input/IA_Look.IA_Look"))
  (Default|RotateCharacter (Variables|Default|GetCharRef) ActionValue))

(event EventBeginPlay)

(event EventTick
  (params (DeltaSeconds :type Float%20%28single-precision%29)))

(event EventPossess
  (params (PossessedPawn :type Pawn%20Object%20Reference))
  (bind _asbp_player_character (Utilities|Casting|CastToBP_PlayerCharacter PossessedPawn))
  (Variables|Default|SetCharRef _asbp_player_character)
  (CallFunction|SetDefaultInputs)
  (Development|PrintString "Hello"))

(fn ConstructionScript)

(fn SetDefaultInputs
  (for _array_element (Utilities|Array|MakeArray "/Game/MyContent/Player/Input/IMC_Movement.IMC_Movement" "/Game/MyContent/Player/Input/IMC_Camera.IMC_Camera")
    (CallFunction|AddInput _array_element 0 true)))

(fn AddInput
  (params (MappingContext :type Input%20Mapping%20Context%20Object%20Reference) (Priority :type Integer) (Options%20Ignore%20All%20Pressed%20Keys%20Until%20Release :type Boolean))
  (Input|AddMappingContext (PlayerController|LocalPlayerSubsystems|GetEnhancedInputLocalPlayerSubsystem) MappingContext Priority (Utilities|Struct|MakeModifyContextOptions Options%20Ignore%20All%20Pressed%20Keys%20Until%20Release false false)))