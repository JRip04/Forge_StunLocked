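; BP_CameraManager is a shared camera actor that frames two players together by following their midpoint and zooming with their separation.
; It binds to BP_GM_Main's camera setup event; InitCamera makes it player 0's view target and registers itself on every BP_PlayerCharacter.
; A fast looping timer, rather than Tick, eases location and clamped spring arm length whenever more than one player controller exists.
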(event Custom|InitCamera
  (Game|Player|SetViewTargetwithBlend (Game|GetPlayerController 0) self 0.0 "VTBlend_Linear" 0.0 false)
  (bind _outactors (Actor|GetAllActorsOfClass "/Game/MyContent/Player/BP_PlayerCharacter.BP_PlayerCharacter_C"))
  (bind _output_get (Variables|Default|SetPlayerArray _outactors))
  (for _array_element _output_get
    (Variables|/Game/MyContent/Player/BP_PlayerCharacter.BP_PlayerCharacter_C|SetCamRef _array_element self))
  (Utilities|Time|SetTimerbyFunctionName 0 "LerpBetweenPlayers" 0.01 true))

(event EventBeginPlay
  (bind _asbp_gm_main (Utilities|Casting|CastToBP_GM_Main (Game|GetGameMode)))
  (EventDispatchers|BindEventtoSetUpCamera _asbp_gm_main (EventDispatchers|CreateEvent :!event Custom|InitCamera)))

(event Collision|EventActorBeginOverlap
  (params (OtherActor :type Actor%20Object%20Reference)))

(event EventTick
  (params (DeltaSeconds :type Float%20%28single-precision%29)))

(fn ConstructionScript)

(fn LerpBetweenPlayers
  (bind _playerarray (Variables|Default|GetPlayerArray))
  (bind _output (Utilities|Array|Get(acopy) _playerarray 1))
  (bind _output_2 (Utilities|Array|Get(acopy) _playerarray))
  (if (> (Class|GameplayStatics|GetNumPlayerControllers) 1)
    (Variables|/Script/Engine.SpringArmComponent|SetTargetArmLength (Variables|Default|GetSpringArm) (Math|Float|Lerp (Variables|/Script/Engine.SpringArmComponent|GetTargetArmLength (Variables|Default|GetSpringArm)) (Math|Float|Clamp(Float) (* (Transformation|GetDistanceTo _output_2 _output) 2.0) 8e+02 1.6e+03) (* (Utilities|Time|GetWorldDeltaSeconds) 3.0)))
    (Transformation|SetActorLocation self (Math|Vector|Lerp(Vector) (Transformation|GetActorLocation) (/ (+ (Transformation|GetActorLocation _output_2) (Transformation|GetActorLocation _output)) 2) (* (Utilities|Time|GetWorldDeltaSeconds) 4.0)) false false)))