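; Player character that moves relative to an external camera actor (CamRef) and turns through controller yaw and pitch.
; MoveCharacter applies axis input along camera-derived vectors and enables orient-to-movement only at zero input; RotateCharacter is gated by CanRotate, which DelayRotate restores after a delay.
; OutOfBounds sharply slows walking when the character strays too far from CamRef.
; Turn-montage and camera-angle experiments remain disconnected; BeginPlay only prints the camera's name.
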(event Custom|DelayRotate
  (params (Duration :type Float%20%28single-precision%29))
  (Utilities|FlowControl|Delay Duration)
  (Variables|Default|SetCanRotate true))

(event EventBeginPlay
  (Utilities|FlowControl|Delay 0.2)
  (Development|PrintString (Utilities|GetDisplayName (Variables|Default|GetCamRef))))

(event Collision|EventActorBeginOverlap
  (params (OtherActor :type Actor%20Object%20Reference)))

(event EventTick
  (params (DeltaSeconds :type Float%20%28single-precision%29)))

(fn ConstructionScript)

(fn MoveCharacter
  (params (Axis :type Vector%202D%20Structure))
  (bind _camref (Variables|Default|GetCamRef))
  (bind _camera (Variables|/Game/MyContent/Player/Input/Camera/BP_CameraManager.BP_CameraManager_C|GetCamera _camref))
  (bind _returnvalue (Transformation|GetWorldRotation _camera))
  (bind _returnvalue_2 (Math|Rotator|MakeRotator (.yaw _returnvalue) 0.0 0.0))
  (bind _output_get (Variables|Default|SetPlayerAxis Axis))
  (Utilities|FlowControl|Sequence
    (:then_0
      (Pawn|Input|AddMovementInput (Math|Vector|GetRightVector _returnvalue_2) (.X (Math|Vector2D|BreakVector2D _output_get)) false))
    (:then_1
      (Pawn|Input|AddMovementInput (Math|Vector|GetForwardVector _returnvalue_2) (.Y (Math|Vector2D|BreakVector2D _output_get)) false))
    (:then_2
      (Variables|/Script/Engine.CharacterMovementComponent|SetbOrientRotationToMovement (Variables|Character|GetCharacterMovement) (<= (Class|KismetMathLibrary|VSize2DSquared _output_get) 0.0)))))

(fn RotateCharacter
  (params (Axis :type Vector%202D%20Structure))
  (Variables|Default|SetPlayerRotateAxis Axis)
  (if (Variables|Default|GetCanRotate)
    (Utilities|FlowControl|Sequence
      (:then_0
        (Pawn|Input|AddControllerYawInput (.x (Variables|Default|GetPlayerRotateAxis))))
      (:then_1
        (Pawn|Input|AddControllerPitchInput (.y (Variables|Default|GetPlayerRotateAxis)))))))

(fn OutOfBounds
  (bind _charactermovement (Variables|Character|GetCharacterMovement))
  (if (> (Math|Vector|Distance(Vector) (Transformation|GetActorLocation (Variables|Default|GetCamRef)) (Transformation|GetActorLocation)) 8e+02)
    (Variables|Default|SetbIsOutOfBounds true)
    (Variables|/Script/Engine.CharacterMovementComponent|SetMaxWalkSpeed _charactermovement 3e+01)
    (else
      (Variables|Default|SetbIsOutOfBounds false)
      (Variables|/Script/Engine.CharacterMovementComponent|SetMaxWalkSpeed _charactermovement 6e+02))))